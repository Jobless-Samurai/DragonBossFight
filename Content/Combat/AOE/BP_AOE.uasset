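; Area-of-effect actor that detects the actors around its location when triggered and reports each one, leaving the effect to listeners.
; Trigger runs a sphere overlap at the configured radius across several object types, optionally ignoring the instigator.
; Each overlapped actor is broadcast through the OnAOEOverlapActor dispatcher; no damage is applied here.
; An optional debug sphere shows the affected area.
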(event `Trigger`
  ; Trigger Event
  (`self.SpawnAOESphere`))

(event `SpawnAOESphere`
  ; SphereAOE_Damage
  (if (`self.Draw Debug AOE Damage Sphere ?`)
    (`KismetSystemLibrary.DrawDebugSphere` (`self.K2_GetActorLocation`) (`self.AOE Damage Sphere Radius`) 12 (struct :`R` 1.0 :`G` 0.058954 :`A` 1.0) 2.0 2.0))
  (bind _outactors (`KismetSystemLibrary.SphereOverlapActors` (`self.K2_GetActorLocation`) (`self.AOE Damage Sphere Radius`) (`|MakeArray` "ObjectTypeQuery3" "ObjectTypeQuery1" "ObjectTypeQuery4" "ObjectTypeQuery5" "ObjectTypeQuery6" "ObjectTypeQuery7" :!type "EObjectTypeQuery Enum") null (`|MakeArray` (select `bool` (`self.Ignore Self ?`) :`true` (`self.GetInstigator`) :!type "Actor Object Reference"))))
  (for _array_element _outactors
    (`self.OnAOE Overlap Actor` _array_element)))

(fn `UserConstructionScript`)