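; BP_Throwable is a throwable explosive actor that detonates either after a delay or on contact.
; Its construction script loads explosive settings from a data table row, which selects the trigger at BeginPlay.
; Contact mode polls a small sphere overlap on a fast looping timer, ignoring itself and its instigator or owner, instead of using collision events.
; Both triggers fire the AOEDamage component, whose overlap event sends TakeDamageMessage to affected actors.
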(event `self.ReceiveBeginPlay`
  ; BeginPlay
  (if (`.IsTimerExplosive?_8_F3906FA8448DA16CD6588FBD1C86226E` (break `/Game/Combat/Throwable/S_ExplosiveInfo` (`self.Explosive Info`)))
    (`self.TimeDelayTrigger`)
    (else
      (`self.HitTrigger`))))

(event `TimeDelayTrigger`
  ; Trigger
  (`KismetSystemLibrary.Delay` (`.ExplosionTimeDelay_12_7545B6FB41E6EC206B4ABE9BF6BC474C` (break `/Game/Combat/Throwable/S_ExplosiveInfo` (`self.Explosive Info`))))
  (`/Game/Combat/AC_AOEDamage.ActivateAOEDamage` (`self.AOEDamage`) (`self.Explosive Info`) (`self.K2_GetActorLocation`) true false (`self.Damage Causer`)))

(event `HitTrigger`
  ; Trigger
  (`KismetSystemLibrary.K2_ClearAndInvalidateTimerHandle` (`self.HitDeact`))
  (bind _returnvalue (`KismetSystemLibrary.K2_SetTimerDelegate` (delegate `UpdateHitTrigger`) 0.01 true))
  (set `self.HitDeact` _returnvalue))

(event `UpdateHitTrigger`
  (bind _returnvalue (`self.GetInstigator`))
  ; Trigger
  (if (`self.ShouldDrawHitSphereOverlap`)
    (`KismetSystemLibrary.DrawDebugSphere` (`self.K2_GetActorLocation`) 20.0 12 (struct :`R` 1.0 :`G` 0.119792 :`B` 0.383156 :`A` 1.0) 4.0 1.0))
  (bind (_outactors _returnvalue_2) (`KismetSystemLibrary.SphereOverlapActors` (`self.K2_GetActorLocation`) 20.0 (`|MakeArray` "ObjectTypeQuery1" "ObjectTypeQuery3" "ObjectTypeQuery4" "ObjectTypeQuery5" "ObjectTypeQuery6" "ObjectTypeQuery7" :!type "EObjectTypeQuery Enum") null (`|MakeArray` self (select `bool` (`KismetSystemLibrary.IsValid` _returnvalue) :`false` (`self.GetOwner`) :`true` _returnvalue :!type "Actor Object Reference") :!type "Actor Object Reference")))
  (if _returnvalue_2
    (`KismetSystemLibrary.K2_ClearAndInvalidateTimerHandle` (`self.HitDeact`))
    (`/Game/Combat/AC_AOEDamage.ActivateAOEDamage` (`self.AOEDamage`) (`self.Explosive Info`) (`self.K2_GetActorLocation`) false false (`self.Damage Causer`))))

(event `self.AOEDamage.OnAOEDamageOverlap`
  (params (`Other Actor` :type "Actor Object Reference"))
  ; Trigger
  (message `/Game/Combat/Damage/I_Damagable.Take Damage` `Other Actor` (`self.Damage Info`) (`self.Damage Causer`)))

(fn `Get Explosive Data`
  (bind _returnvalue (`|GetDataTableRow` (`self.Explosive Data`) (`self.Explosive Name`))
    (:`then`
      (set `self.Explosive Info` _returnvalue)
      (return))))

(fn `UserConstructionScript`
  (`self.Get Explosive Data`))