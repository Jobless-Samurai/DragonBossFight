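; AC_AOEDamage is an actor component that handles an explosion's area-of-effect hit detection, effects and sound.
; ActivateAOEDamage stores the explosion info and location, then triggers a sphere overlap with optional debug drawing and self-ignore.
; Each overlapped actor is broadcast through OnAOEDamageOverlap, leaving damage application to listeners.
; The owning actor is then destroyed, and the explosion emitter and sound spawn at the blast location.
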(event `ActivateAOEDamage`
  (params (`Explosion Info` :type "/Game/Combat/Throwable/S_ExplosiveInfo Structure") (`Explosion Location` :type "Vector Structure") (`Draw Debug AOE Damage Sphere ?` :type Boolean) (`Ignore Self ?` :type Boolean) (`Self Actor` :type "Actor Object Reference"))
  ; Setup Variables and Trigger Event
  (set `self.Explosive Info` `Explosion Info`)
  (set `self.Explosion Location` `Explosion Location`)
  (set `self.Draw Debug AOE Damage Sphere ?` `Draw Debug AOE Damage Sphere ?`)
  (set `self.Ignore Self ?` `Ignore Self ?`)
  (set `self.Self Actor` `Self Actor`)
  (`self.Trigger`))

(event `Trigger`
  ; Trigger Event
  (`self.SpawnAOESphere`)
  (`self.SpawnExplosiveFXSound`))

(event `SpawnAOESphere`
  (bind ((`AOEDamageSphereRadius_11_96100B4F4394CB2B4E23BDA13CAAED1F` _aoedamagesphereradius)) (break `/Game/Combat/Throwable/S_ExplosiveInfo` (`self.Explosive Info`)))
  ; SphereAOE_Damage
  (if (`self.Draw Debug AOE Damage Sphere ?`)
    (`KismetSystemLibrary.DrawDebugSphere` (`self.Explosion Location`) _aoedamagesphereradius 12 (struct :`G` 1.0 :`B` 0.839328 :`A` 1.0) 10.0 2.0))
  (bind _outactors (`KismetSystemLibrary.SphereOverlapActors` (`self.Explosion Location`) _aoedamagesphereradius (`|MakeArray` "ObjectTypeQuery3" "ObjectTypeQuery1" "ObjectTypeQuery4" "ObjectTypeQuery5" "ObjectTypeQuery6" "ObjectTypeQuery7" :!type "EObjectTypeQuery Enum") null (`|MakeArray` (`self.GetOwner`) (select `bool` (`self.Ignore Self ?`) :`true` (`self.Self Actor`)))))
  (for _array_element _outactors
    (`self.OnAOEDamageOverlap` _array_element))
  (`Actor.K2_DestroyActor` (`self.GetOwner`)))

(event `SpawnExplosiveFXSound`
  (bind (_explosionfx _explosionsound) (break `/Game/Combat/Throwable/S_ExplosiveInfo` (`self.Explosive Info`)))
  ; Visuals
  (`GameplayStatics.SpawnEmitterAtLocation` _explosionfx (`self.Explosion Location`))
  (`GameplayStatics.PlaySoundAtLocation` _explosionsound (`self.Explosion Location`) (struct) 1.0 1.0 0.0 null null null null))