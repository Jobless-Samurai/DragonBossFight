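; BP_Enemy_PatrolRoute is a patrol route helper that supplies waypoints for enemy AI from the points of a spline.
; GetSplineLocation returns the world location of the spline point at the current PatrolIndex.
; IncreamentIndex steps the index by Direction and flips that direction at the last and first points, so the route is traversed back and forth rather than looped.
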(fn `Get Spline Location`
  (returns (Location :type "Vector Structure"))
  (return (`SplineComponent.GetLocationAtSplinePoint` (`self.PatrolRoute`) (`self.Patrol index`) "World")))

(fn `Increament Index`
  (set `self.Patrol index` (+ (`self.Patrol index`) (`self.Direction`)))
  (if (== (`self.Patrol index`) (- (`SplineComponent.GetNumberOfSplinePoints` (`self.PatrolRoute`)) 1))
    (set `self.Direction` -1)
    (elif (== (`self.Patrol index`) 0)
      (set `self.Direction` 1))))

(fn `UserConstructionScript`)